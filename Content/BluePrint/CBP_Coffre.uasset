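; CBP_Coffre is a puzzle chest Blueprint that rotates Cube1 when its referenced lights are all lit in the correct order.
; It binds to each light's on/off events to count lit lights, while exposed events append or remove letters in a string.
; When all are lit, a string matching Sequence triggers the rotation; otherwise it clears its state and calls CoffreEteint on every light.
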(event Custom|CustomEvent_0
  (Transformation|SetRelativeRotation (Variables|Default|GetCube1) "90.000000,90.000000, 0" false false))

(event Custom|LumiereAllumee
  (bind _output_get (Variables|Default|SetNmbreLumieresAllumees (+ (Variables|Default|GetNmbreLumieresAllumees) 1)))
  (Development|PrintString (Utilities|String|Append (Utilities|String|ToString(Integer) _output_get) (Variables|Default|GetLettres)))
  (if (== _output_get (Utilities|Array|Length (Variables|Default|GetRefCBPLumiere)))
    (if (Utilities|Enum|Equal(Enum) (Variables|Default|GetLettres) (Variables|Default|GetSequence))
      (Development|PrintString "Bon")
      (Transformation|SetRelativeRotation (Variables|Default|GetCube1) "90.000000,90.000000, 0" false false)
      (else
        (Variables|Default|SetNmbreLumieresAllumees 0)
        (Variables|Default|SetLettres "")
        (for _array_element (Variables|Default|GetRefCBPLumiere)
          (Default|CoffreEteint _array_element))))))

(event Custom|LumiereEteinte
  (Variables|Default|SetNmbreLumieresAllumees (- (Variables|Default|GetNmbreLumieresAllumees) 1)))

(event EventBeginPlay
  (|CallParentFunction)
  (for _array_element (Variables|Default|GetRefCBPLumiere)
    (EventDispatchers|BindEventtoLumiereAllumee _array_element (delegate Custom|LumiereAllumee))
    (EventDispatchers|BindEventtoLumiereEteinte _array_element (delegate Custom|LumiereEteinte))))

(event Collision|EventActorBeginOverlap
  (params (OtherActor :type Actor%20Object%20Reference))
  (|CallParentFunction OtherActor) ; This node is disabled and will not be called.\nDrag off pins to build functionality.
)

(event EventTick
  (params (DeltaSeconds :type Float%20%28single-precision%29))
  (|CallParentFunction DeltaSeconds) ; This node is disabled and will not be called.\nDrag off pins to build functionality.
)

(event EventFuncEchangeLettre
  (params (EchangeLettre :type String))
  (Variables|Default|SetLettres (Utilities|String|Append (Variables|Default|GetLettres) EchangeLettre)))

(event EventFuncSupprLettre
  (params (EffaceLettre :type String))
  (Variables|Default|SetLettres (Utilities|String|Replace (Variables|Default|GetLettres) EffaceLettre)))

(fn ConstructionScript
  (|CallParentFunction))