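; Stone pedestal actor that collects the red, green and blue stones carried by BP_Rosa and serves as a win condition.
; An in-range ActionInterraction flags the stones held in the player's InvPierre, then empties that inventory, so deposits accumulate across visits.
; Once all three flags are set, it prints a win message and calls AllumeFeu.
; Tick mirrors each flag onto its matching component's visibility, all hidden at BeginPlay.
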(event EventBeginPlay
  (|CallParentFunction)
  (Rendering|SetVisibility (Variables|Default|GetL_rouge) false true)
  (Variables|Default|SetV_bleue false)
  (Variables|Default|SetV_rouge false)
  (Variables|Default|SetV_vert false))

(event Collision|EventActorBeginOverlap
  (params (OtherActor :type Actor%20Object%20Reference))
  (|CallParentFunction OtherActor) ; This node is disabled and will not be called.\nDrag off pins to build functionality.
)

(event EventTick
  (params (DeltaSeconds :type Float%20%28single-precision%29))
  (|CallParentFunction DeltaSeconds)
  (Rendering|SetVisibility (Variables|Default|GetL_bleue) (Variables|Default|GetV_bleue) true)
  (Rendering|SetVisibility (Variables|Default|GetL_Vert) (Variables|Default|GetV_vert) true)
  (Rendering|SetVisibility (Variables|Default|GetL_rouge) (Variables|Default|GetV_rouge) true))

(event EventActionInterraction
  (params (dist :type Float%20%28single-precision%29))
  (if (<= dist 2e+02)
    (bind _asbp_rosa (Utilities|Casting|CastToBP_Rosa (Game|GetPlayerCharacter 0)))
    (if (.Bleu (Utilities|Struct|BreakStruct_invPierre (Variables|/Game/Personnage/Rosa/BP_Rosa.BP_Rosa_C|Getinv_pierre _asbp_rosa)))
      (Variables|Default|SetV_bleue true))
    (if (.Vert (Utilities|Struct|BreakStruct_invPierre (Variables|/Game/Personnage/Rosa/BP_Rosa.BP_Rosa_C|Getinv_pierre _asbp_rosa)))
      (Variables|Default|SetV_vert true))
    (if (.Rouge (Utilities|Struct|BreakStruct_invPierre (Variables|/Game/Personnage/Rosa/BP_Rosa.BP_Rosa_C|Getinv_pierre _asbp_rosa)))
      (Variables|Default|SetV_rouge true))
    (Variables|/Game/Personnage/Rosa/BP_Rosa.BP_Rosa_C|Setinv_pierre _asbp_rosa (Utilities|Struct|MakeStruct_invPierre false false false))
    (if (Variables|Default|GetV_bleue)
      (if (Variables|Default|GetV_rouge)
        (if (Variables|Default|GetV_vert)
          (Development|PrintString "YOU WIN")
          (Default|CallAllumeFeu))))))

(fn ConstructionScript
  (|CallParentFunction))