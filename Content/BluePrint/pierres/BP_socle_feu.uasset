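; BP_socle_feu is a fire pedestal whose PFire effect lights when a stone pedestal signals it, an event named as the end of the game.
; On BeginPlay it finds every BP_socle_pierre actor and binds its Fin_du_game event to each one's AllumeFeu dispatcher.
; Any single broadcast activates PFire without a reset, with no counting or other condition in this Blueprint.
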(event Custom|fin_du_game
  (Components|Activation|Activate (Variables|Default|GetP_Fire) false))

(event EventBeginPlay
  (|CallParentFunction)
  (bind _outactors (Actor|GetAllActorsOfClass "/Game/BluePrint/pierres/BP_socle_pierre.BP_socle_pierre_C"))
  (for _array_element _outactors
    (EventDispatchers|BindEventtoAllumeFeu _array_element (delegate Custom|fin_du_game))))

(event Collision|EventActorBeginOverlap
  (params (OtherActor :type Actor%20Object%20Reference))
  (|CallParentFunction OtherActor) ; This node is disabled and will not be called.\nDrag off pins to build functionality.
)

(event EventTick
  (params (DeltaSeconds :type Float%20%28single-precision%29))
  (|CallParentFunction DeltaSeconds) ; This node is disabled and will not be called.\nDrag off pins to build functionality.
)

(fn ConstructionScript
  (|CallParentFunction))