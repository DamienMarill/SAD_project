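; Blue stone pickup that the player collects into the stone inventory of BP_Rosa.
; ActionInterraction checks that the distance is within Portee and that PierreIci is still true, then clears the flag and hides Box with its children.
; It then casts the player character to BP_Rosa, sets Bleu in InvPierre while keeping Vert and Rouge, and plays the Verre sound.
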(event EventBeginPlay
  (|CallParentFunction))

(event Collision|EventActorBeginOverlap
  (params (OtherActor :type Actor%20Object%20Reference))
  (|CallParentFunction OtherActor))

(event EventTick
  (params (DeltaSeconds :type Float%20%28single-precision%29))
  (|CallParentFunction DeltaSeconds) ; This node is disabled and will not be called.\nDrag off pins to build functionality.
)

(event EventActionInterraction
  (params (dist :type Float%20%28single-precision%29))
  (if (<= dist (Variables|Default|Getportee))
    (if (Variables|Default|Getpierre_ici)
      (bind _output_get (Variables|Default|Setpierre_ici false))
      (Rendering|SetVisibility (Variables|Default|GetBox) _output_get true)
      (bind _asbp_rosa (Utilities|Casting|CastToBP_Rosa (Game|GetPlayerCharacter 0)))
      (Variables|/Game/Personnage/Rosa/BP_Rosa.BP_Rosa_C|Setinv_pierre _asbp_rosa (Utilities|Struct|MakeStruct_invPierre true (.Vert (Utilities|Struct|BreakStruct_invPierre (Variables|/Game/Personnage/Rosa/BP_Rosa.BP_Rosa_C|Getinv_pierre _asbp_rosa))) (.Rouge (Utilities|Struct|BreakStruct_invPierre (Variables|/Game/Personnage/Rosa/BP_Rosa.BP_Rosa_C|Getinv_pierre _asbp_rosa)))))
      (Audio|PlaySound2D "/Game/sons/verre.verre" 1.0 1.0 0.0 0 0))))

(fn ConstructionScript
  (|CallParentFunction))