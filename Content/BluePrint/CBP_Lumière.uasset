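; CBP_Lumière is a light actor toggled by a linked switch, with each light tied to a letter on a chest.
; At BeginPlay it binds JourNuit to the switch, which flips the point light between zero and its set intensity.
; Each toggle passes its letter to the chest's swap (on) or remove (off) function and fires a matching dispatcher.
; CoffreEteint turns the light off without updating the chest or firing dispatchers.
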(event Custom|JourNuit
  ;[1 1 1] Allumer la lumière
  (Development|PrintString "Hello")
  (if (Variables|Default|GetLumièreAllumee)
    (CallFunction|Eteinde)
    (Default|FuncSupprLettre (Variables|Default|GetRefCoffre) (Variables|Default|GetLettre))
    (Default|CallLumiereEteinte)
    (else
      (CallFunction|Allumer)
      (Default|FuncEchangeLettre (Variables|Default|GetRefCoffre) (Variables|Default|GetLettre))
      (Default|CallLumiereAllumee))))

(event Custom|CoffreEteint
  (CallFunction|Eteinde))

(event EventBeginPlay
  ;[1 1 1] Allumer la lumière
  (EventDispatchers|BindEventtoInterupteur (Variables|Default|GetCBP_Interrupteur_Ref) (delegate Custom|JourNuit)))

(event Collision|EventActorBeginOverlap
  (params (OtherActor :type Actor%20Object%20Reference))
  (|CallParentFunction OtherActor) ; This node is disabled and will not be called.\nDrag off pins to build functionality.
)

(event EventTick
  (params (DeltaSeconds :type Float%20%28single-precision%29))
  (|CallParentFunction DeltaSeconds) ; This node is disabled and will not be called.\nDrag off pins to build functionality.
)

(fn ConstructionScript
  (|CallParentFunction))

(fn Eteinde
  (Rendering|Components|Light|SetIntensity (Variables|Default|GetPointLight) 0.0)
  (Variables|Default|SetLumièreAllumee false))

(fn Allumer
  (Rendering|Components|Light|SetIntensity (Variables|Default|GetPointLight) (Variables|Default|GetIntensitéLumière))
  (Variables|Default|SetLumièreAllumee true))