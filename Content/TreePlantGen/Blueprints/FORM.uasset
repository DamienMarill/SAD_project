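; FORM is a spline shape Blueprint, apparently for tree and plant generation, that previews a tapered chain of spline meshes in its Construction Script.
; Unlocked, it pins the first two spline points, picks a random MeshPool mesh per segment and records points, tangents and meshes into DATA.
; With LOCK on, it rebuilds the spline and same meshes from DATA, freezing the result.
; Segment scale shrinks linearly along the spline.
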(event EventBeginPlay)

(event Collision|EventActorBeginOverlap
  (params (OtherActor :type Actor%20Object%20Reference)))

(event EventTick
  (params (DeltaSeconds :type Float%20%28single-precision%29)))

(fn ConstructionScript
  (bind _spline (Variables|Default|GetSpline))
  (bind _data (Variables|Default|GetDATA))
  (bind _data_2 (Variables|Default|GetDATA))
  (bind _data_3 (Variables|Default|GetDATA))
  (bind _spline_2 (Variables|Default|GetSpline))
  (if (Variables|Default|GetLOCK)
    (Utilities|FlowControl|Sequence
      (:then_0
        (Spline|ClearSplinePoints (Variables|Default|GetSpline) false)
        (for (_array_element _array_index) (.splinepoints _data)
          (Spline|AddSplinePoint _spline _array_element "Local" false)
          (Spline|SetTangentatSplinePoint _spline _array_index (Utilities|Array|Get(acopy) (.splinepoints_tangents _data) _array_index) "Local" false))
        (Spline|UpdateSpline (Variables|Default|GetSpline)))
      (:then_1
        (LocalVariables|SetscaleStep (|((1.000000/meshCount)-({7F89FFA3-480C-7F44-8F9F-76AE85199B69}/meshCount)) (Math|Conversions|ToFloat(Integer) (- (Spline|GetNumberOfSplinePoints (Variables|Default|GetSpline)) 1))))
        (for (_array_element_2 _array_index_2) (.meshsections (Variables|Default|GetDATA))
          (LocalVariables|Seti _array_index_2)
          (bind _returnvalue (AddComponent|AddSplineMeshComponent false))
          (Components|StaticMesh|SetStaticMesh _returnvalue _array_element_2)
          (Rendering|Material|SetMaterial _returnvalue 0 (Variables|Default|GetPreviewMaterial))
          (SplineMesh|SetSplineUpDir _returnvalue (Math|Vector|MakeVector 0.5 -0.4 0.0) false)
          (SplineMesh|SetStartandEnd _returnvalue (.Location (Spline|GetLocationandTangentatSplinePoint (Variables|Default|GetSpline) (LocalVariables|Geti) "Local")) (.Tangent (Spline|GetLocationandTangentatSplinePoint (Variables|Default|GetSpline) (LocalVariables|Geti) "Local")) (.Location (Spline|GetLocationandTangentatSplinePoint (Variables|Default|GetSpline) (+ (LocalVariables|Geti) 1) "Local")) (.Tangent (Spline|GetLocationandTangentatSplinePoint (Variables|Default|GetSpline) (+ (LocalVariables|Geti) 1) "Local")) false :!class /Script/Engine.SplineMeshComponent) ; ... + Fix for the last point being misplaced due to last long tangent (UE bug?)
          (SplineMesh|SetStartScale _returnvalue (Math|Vector2D|MakeVector2D (- 1.0 (* (LocalVariables|Geti) (LocalVariables|GetscaleStep))) (- 1.0 (* (LocalVariables|Geti) (LocalVariables|GetscaleStep)))) false :!class /Script/Engine.SplineMeshComponent)
          (SplineMesh|SetEndScale _returnvalue (Math|Vector2D|MakeVector2D (- 1.0 (* (+ (LocalVariables|Geti) 1) (LocalVariables|GetscaleStep))) (- 1.0 (* (+ (LocalVariables|Geti) 1) (LocalVariables|GetscaleStep)))) true :!class /Script/Engine.SplineMeshComponent))))
    (else
      (Utilities|Array|Clear (.splinepoints _data_2))
      (Utilities|Array|Clear (.splinepoints_tangents _data_2))
      (Utilities|Array|Clear (.meshsections _data_2))
      (Spline|SetLocationatSplinePoint (Variables|Default|GetSpline) 0 (Math|Vector|MakeVector 0.0 0.0 0.0) "Local" false)
      (Spline|SetLocationatSplinePoint (Variables|Default|GetSpline) 1 (Variables|Default|GetFirstPointOffset) "Local" true)
      (LocalVariables|SetscaleStep (|((1.000000/meshCount)-({7F89FFA3-480C-7F44-8F9F-76AE85199B69}/meshCount)) (Math|Conversions|ToFloat(Integer) (- (Spline|GetNumberOfSplinePoints (Variables|Default|GetSpline)) 1))))
      (for _index (range 0 (- (Spline|GetNumberOfSplinePoints (Variables|Default|GetSpline)) 2))
        (LocalVariables|Seti _index)
        (bind _returnvalue_2 (AddComponent|AddSplineMeshComponent false))
        (Components|StaticMesh|SetStaticMesh _returnvalue_2 (Utilities|Array|Get(acopy) (Variables|Default|GetMeshPool) (Math|Random|RandomInteger (Utilities|Array|Length (Variables|Default|GetMeshPool)))))
        (Rendering|Material|SetMaterial _returnvalue_2 0 (Variables|Default|GetPreviewMaterial))
        (SplineMesh|SetSplineUpDir _returnvalue_2 (Math|Vector|MakeVector 0.5 -0.4 0.0) false)
        (SplineMesh|SetStartandEnd _returnvalue_2 (.Location (Spline|GetLocationandTangentatSplinePoint (Variables|Default|GetSpline) (LocalVariables|Geti) "Local")) (.Tangent (Spline|GetLocationandTangentatSplinePoint (Variables|Default|GetSpline) (LocalVariables|Geti) "Local")) (.Location (Spline|GetLocationandTangentatSplinePoint (Variables|Default|GetSpline) (+ (LocalVariables|Geti) 1) "Local")) (.Tangent (Spline|GetLocationandTangentatSplinePoint (Variables|Default|GetSpline) (+ (LocalVariables|Geti) 1) "Local")) false :!class /Script/Engine.SplineMeshComponent)
        (SplineMesh|SetStartScale _returnvalue_2 (Math|Vector2D|MakeVector2D (- 1.0 (* (LocalVariables|Geti) (LocalVariables|GetscaleStep))) (- 1.0 (* (LocalVariables|Geti) (LocalVariables|GetscaleStep)))) false :!class /Script/Engine.SplineMeshComponent)
        (SplineMesh|SetEndScale _returnvalue_2 (Math|Vector2D|MakeVector2D (- 1.0 (* (+ (LocalVariables|Geti) 1) (LocalVariables|GetscaleStep))) (- 1.0 (* (+ (LocalVariables|Geti) 1) (LocalVariables|GetscaleStep)))) true :!class /Script/Engine.SplineMeshComponent)
        (Utilities|Array|Add (.meshsections (Variables|Default|GetDATA)) (Variables|/Script/Engine.StaticMeshComponent|GetStaticMesh _returnvalue_2)))
      (for _index_2 (range 0 (- (Spline|GetNumberOfSplinePoints _spline_2) 1))
        (Utilities|Array|Add (.splinepoints _data_3) (Spline|GetLocationatSplinePoint _spline_2 _index_2 "Local"))
        (Utilities|Array|Add (.splinepoints_tangents _data_3) (Spline|GetTangentatSplinePoint _spline_2 _index_2 "Local"))))))