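; LianaAdder hangs a cable-component liana between two selected Tree branches, storing their owners and indices at construction and spawning the cable at BeginPlay.
; A looping timer recomputes both ends through each branch's OffsetVectorSameAsInGPU, with timelines lerping between updates; a missing branch then destroys the actor.
; A sphere trigger hides the cable, slows its tick and stops updates when the view target leaves.
; Briefly raised solver iterations smooth out startup jitter.
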(event OnComponentBeginOverlap(CullTrigger)
  (params (OverlappedComponent :type Primitive%20Component%20Object%20Reference) (OtherActor :type Actor%20Object%20Reference) (OtherComp :type Primitive%20Component%20Object%20Reference) (OtherBodyIndex :type Integer) (bFromSweep :type Boolean) (SweepResult :type Hit%20Result%20Structure%20%28by%20ref%29))
  (bind _activeliana (Variables|Default|GetactiveLiana))
  (if (== OtherActor (Pawn|GetViewTarget (Game|GetPlayerController 0)))
    (Development|SetHiddeninGame _activeliana false false)
    (Class|ActorComponent|SetComponentTickInterval _activeliana 0.0)
    (CallFunction|UpdateLianaEndsON/OFF true)))

(event OnComponentEndOverlap(CullTrigger)
  (params (OverlappedComponent :type Primitive%20Component%20Object%20Reference) (OtherActor :type Actor%20Object%20Reference) (OtherComp :type Primitive%20Component%20Object%20Reference) (OtherBodyIndex :type Integer))
  (bind _activeliana (Variables|Default|GetactiveLiana))
  (if (== OtherActor (Pawn|GetViewTarget (Game|GetPlayerController 0)))
    (Development|SetHiddeninGame _activeliana true false)
    (Class|ActorComponent|SetComponentTickInterval _activeliana 5.0)
    (CallFunction|UpdateLianaEndsON/OFF false)))

(event Custom|UpdateLianaEnds
  (bind _endactivebranch (Variables|Default|GetendActiveBranch))
  (bind _startactivebranch (Variables|Default|GetstartActiveBranch))
  (Utilities|IsValid (Variables|Default|GetendActiveBranch)
    (:Is%20Valid
      (Utilities|FlowControl|Sequence
        (:then_0
          (bind _vectorwithoffset (Default|OffsetVectorSameasinGPU _endactivebranch (Math|Transform|TransformLocation (Transformation|GetActorTransform (Variables|Default|GetendActiveBranch)) (Variables|Default|GetoriginalEndLoc))))
          (Variables|Default|SetupdatedEndLoc (Math|Transform|InverseTransformLocation (Transformation|GetActorTransform _endactivebranch) _vectorwithoffset))
          (bind _lerp (Timeline|LianaEndLocLerp PlayFromStart)
            (:Update
              (Variables|/Script/CableComponent.CableComponent|SetEndLocation (Variables|Default|GetactiveLiana) (Math|Vector|Lerp(Vector) (Variables|Default|GetcurrentLianaEndLoc) (Variables|Default|GetupdatedEndLoc) _lerp)))
            (:Finished
              (Variables|Default|SetcurrentLianaEndLoc (Variables|Default|GetupdatedEndLoc)))))
        (:then_1
          (Utilities|IsValid (Variables|Default|GetstartActiveBranch)
            (:Is%20Valid
              (bind _vectorwithoffset_2 (Default|OffsetVectorSameasinGPU _startactivebranch (Math|Transform|TransformLocation (Transformation|GetActorTransform (Variables|Default|GetstartActiveBranch)) (Variables|Default|GetoriginalStartLoc))))
              (Variables|Default|SetupdatedStartLoc (Math|Transform|InverseTransformLocation (Transformation|GetActorTransform _startactivebranch) _vectorwithoffset_2))
              (bind _lerp_2 (Timeline|LianaStartLocLerp PlayFromStart)
                (:Update
                  (Transformation|SetRelativeLocation (Variables|Default|GetactiveLiana) (Math|Vector|Lerp(Vector) (Variables|Default|GetcurrentLianaStartLoc) (Variables|Default|GetupdatedStartLoc) _lerp_2) false false))
                (:Finished
                  (Variables|Default|SetcurrentLianaStartLoc (Variables|Default|GetupdatedStartLoc)))))
            (:Is%20Not%20Valid
              (Actor|DestroyActor))))))
    (:Is%20Not%20Valid
      (Actor|DestroyActor))))

(event Custom|UpdateLianaEnds_ON/OFF
  (params (ON/OFF :type Boolean))
  (if ON/OFF
    (bind _returnvalue (Utilities|Time|SetTimerbyEvent (delegate Custom|UpdateLianaEnds) (* (Variables|Lianas|GetanimationUpdateInterval) 1.05) true))
    (Variables|Default|Settimer_UpdateLianaEnds _returnvalue)
    (else
      (Utilities|Time|ClearandInvalidateTimerbyHandle (Variables|Default|Gettimer_UpdateLianaEnds)))))

(event EventBeginPlay
  (bind _lianasettings (Variables|Lianas|GetlianaSettings))
  (bind (_offsetonstartbranch _offsetonendbranch _lianalength _lianawidth _lianastiffness _material) (Utilities|Struct|BreaklianaSettings _lianasettings))
  (Utilities|FlowControl|Sequence
    (:then_0
      (Variables|Default|SetstartActiveBranch (Utilities|Array|Get(acopy) (Variables|/Game/TreePlantGen/Blueprints/InternalLogic/Tree.Tree_C|GetactiveBranches (Variables|Default|GetLianaStartOwner)) (Variables|Default|GetLianaStartBranchIndex)))
      (Variables|Default|SetendActiveBranch (Utilities|Array|Get(acopy) (Variables|/Game/TreePlantGen/Blueprints/InternalLogic/Tree.Tree_C|GetactiveBranches (Variables|Default|GetLianaEndOwner)) (Variables|Default|GetLianaEndBranchIndex)))
      (if (and (Utilities|IsValid (Variables|Default|GetstartActiveBranch)) (Utilities|IsValid (Variables|Default|GetendActiveBranch)))
        (bind _output_get (Variables|Default|SetcurrentLianaStartLoc (Spline|GetLocationatTime (Variables|/Game/TreePlantGen/Blueprints/InternalLogic/Branch.Branch_C|GetSpline (Variables|Default|GetstartActiveBranch)) _offsetonstartbranch "Local" true)))
        (bind _output_get_2 (Variables|Default|SetoriginalStartLoc _output_get))
        (bind _returnvalue (AddComponent|AddCableComponent true (Math|Conversions|ToTransform(Vector) _output_get_2)))
        (bind _output_get_3 (Variables|Default|SetactiveLiana _returnvalue))
        (Transformation|AttachComponentToComponent _output_get_3 (Variables|/Game/TreePlantGen/Blueprints/InternalLogic/Branch.Branch_C|GetDefaultSceneRoot (Variables|Default|GetstartActiveBranch)) "None" "KeepRelative" "KeepRelative" "KeepRelative" true)
        (Rendering|Material|SetMaterial (Variables|Default|GetactiveLiana) 0 _material)
        (Variables|/Script/CableComponent.CableComponent|SetCableLength (Variables|Default|GetactiveLiana) _lianalength)
        (Variables|/Script/CableComponent.CableComponent|SetCableWidth (Variables|Default|GetactiveLiana) _lianawidth)
        (Variables|/Script/CableComponent.CableComponent|SetSolverIterations (Variables|Default|GetactiveLiana) 44) ; BeginPlay liana 'rage' smooth out
        (Variables|Default|SetlianaStiffness _lianastiffness)
        (Class|CableComponent|SetAttachEndto (Variables|Default|GetactiveLiana) (Variables|Default|GetendActiveBranch) "None" "None")
        (bind _output_get_4 (Variables|/Script/CableComponent.CableComponent|SetEndLocation (Variables|Default|GetactiveLiana) (Spline|GetLocationatTime (Variables|/Game/TreePlantGen/Blueprints/InternalLogic/Branch.Branch_C|GetSpline (Variables|Default|GetendActiveBranch)) _offsetonendbranch "Local" true)))
        (bind _output_get_5 (Variables|Default|SetcurrentLianaEndLoc _output_get_4))
        (Variables|Default|SetoriginalEndLoc _output_get_5)
        (Development|SetHiddeninGame (Variables|Default|GetactiveLiana) (> (Transformation|GetDistanceTo (Pawn|GetViewTarget (Game|GetPlayerController 0))) (Variables|Lianas|GetcullDistance)) false)
        (else
          (Development|PrintString (Utilities|String|Append "Liana connection missing! Please select both start & end branch for liana connection.  
Incorrect Liana Manager actor:   " (Utilities|GetObjectName self)) true true "(R=0.895000,G=0.216541,B=0.000000,A=1.000000)" 1e+01))))
    (:then_1
      (Utilities|FlowControl|Delay (Variables|Lianas|GetanimationUpdateInterval))
      (Components|Sphere|SetSphereRadius (Variables|Default|GetCullTrigger) (Variables|Lianas|GetcullDistance) false)
      (Components|Timeline|SetPlayRate (Variables|Default|GetLianaEndLocLerp) (/ 1.0 (Variables|Lianas|GetanimationUpdateInterval)))
      (CallFunction|UpdateLianaEndsON/OFF true))
    (:then_2
      (Utilities|FlowControl|Delay 0.5) ; Because first it's set to very high, to cure the liana 'rage'
      (Variables|/Script/CableComponent.CableComponent|SetSolverIterations (Variables|Default|GetactiveLiana) (Variables|Default|GetlianaStiffness)))))

(fn ConstructionScript
  (bind _lianasettings (Variables|Lianas|GetlianaSettings))
  (bind _lianasettings_2 (Variables|Lianas|GetlianaSettings))
  (bind (_startbranch _endbranch) (Utilities|Struct|BreaklianaSettings _lianasettings))
  (bind (_startbranch_2 _endbranch_2) (Utilities|Struct|BreaklianaSettings _lianasettings_2))
  (if (not (or (not (Utilities|IsValid _startbranch)) (not (Utilities|IsValid _endbranch))))
    (bind _astree (Utilities|Casting|CastToTree (Components|GetOwner (Class|Actor|GetParentComponent _startbranch_2))))
    (Variables|Default|SetLianaStartOwner _astree)
    (bind (_array_element _array_index) (Utilities|Array|ForEachLoopwithBreak (Variables|/Game/TreePlantGen/Blueprints/InternalLogic/Tree.Tree_C|GetactiveBranches _astree) :!label _label)
      (:LoopBody
        (if (== _array_element _startbranch_2)
          (Variables|Default|SetLianaStartBranchIndex _array_index)
          (goto _label Break)))
      (:Completed
        (bind _astree_2 (Utilities|Casting|CastToTree (Components|GetOwner (Class|Actor|GetParentComponent _endbranch_2))))
        (Variables|Default|SetLianaEndOwner _astree_2)
        (bind (_array_element_2 _array_index_2) (Utilities|Array|ForEachLoopwithBreak (Variables|/Game/TreePlantGen/Blueprints/InternalLogic/Tree.Tree_C|GetactiveBranches _astree_2) :!label _label_2)
          (:LoopBody
            (if (== _endbranch_2 _array_element_2)
              (Variables|Default|SetLianaEndBranchIndex _array_index_2)
              (goto _label_2 Break))))))))