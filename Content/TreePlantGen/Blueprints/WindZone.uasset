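; WindZone is a spherical area actor that controls wind animation on the Tree actors inside it.
; Shortly after BeginPlay it claims overlapping trees not already under zone control, starts their animation-cull checks, then sets its collision to ignore.
; Speed, strength and direction events update the zone, with direction stored as actor rotation.
; Only trees within animation range receive changes immediately, avoiding lag spikes; others pick up current values when un-culled.
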(event Custom|ChangeStrength
  (params (newStrength :type Float%20%28single-precision%29))
  ;[1 1 1] Change Speed/Strength/Direction functions for assigned trees.
  ; Only for trees that are in animation range, to avoid lag spike. All other trees will be 'awaken' by un-cull animation function
  ; which is always feed by current WindZone properties, so they'll reflect the wind change after un-culling their animation.
  (Variables|Default|SetwindStrength_[inDegrees] newStrength)
  (for _array_element (Variables|Default|GetassignedTrees)
    (if (Variables|/Game/TreePlantGen/Blueprints/InternalLogic/Tree.Tree_C|GetisInAnimCullDistance _array_element)
      (Default|ChangeWindStrengthonOpportunity _array_element (Variables|Default|GetwindStrength_[inDegrees])))))

(event Custom|ChangeSpeed
  (params (newSpeed :type Float%20%28single-precision%29))
  ;[1 1 1] Change Speed/Strength/Direction functions for assigned trees.
  ; Only for trees that are in animation range, to avoid lag spike. All other trees will be 'awaken' by un-cull animation function
  ; which is always feed by current WindZone properties, so they'll reflect the wind change after un-culling their animation.
  (Variables|Default|SetwindSpeed newSpeed)
  (for _array_element (Variables|Default|GetassignedTrees)
    (if (Variables|/Game/TreePlantGen/Blueprints/InternalLogic/Tree.Tree_C|GetisInAnimCullDistance _array_element)
      (Default|ChangeWindSpeedonOpportunity _array_element (Variables|Default|GetwindSpeed)))))

(event Custom|ChangeDirection
  (params (NewDirection :type Vector))
  ;[1 1 1] Change Speed/Strength/Direction functions for assigned trees.
  ; Only for trees that are in animation range, to avoid lag spike. All other trees will be 'awaken' by un-cull animation function
  ; which is always feed by current WindZone properties, so they'll reflect the wind change after un-culling their animation.
  (Transformation|SetActorRotation (Math|Conversions|RotationFromXVector NewDirection))
  (for _array_element (Variables|Default|GetassignedTrees)
    (if (Variables|/Game/TreePlantGen/Blueprints/InternalLogic/Tree.Tree_C|GetisInAnimCullDistance _array_element)
      (Default|ChangeWindDirectiononOpportunity _array_element NewDirection))))

(event EventBeginPlay
  (Utilities|FlowControl|Delay 0.1) ; Important - it must wait for camera controller to make 'IsInCameraViewRange' work ok
  (for _array_element (Collision|GetOverlappingActors (Variables|Default|GetZone) "/Game/TreePlantGen/Blueprints/InternalLogic/Tree.Tree_C" :!class /Script/Engine.PrimitiveComponent)
    (bind _astree (Utilities|Casting|CastToTree _array_element))
    (if (not (Variables|/Game/TreePlantGen/Blueprints/InternalLogic/Tree.Tree_C|GetisUnderWindZoneControl _astree))
      (Utilities|Array|AddUnique (Variables|Default|GetassignedTrees) _astree)
      (Variables|/Game/TreePlantGen/Blueprints/InternalLogic/Tree.Tree_C|SetassignedWindZone _astree self)
      (Variables|/Game/TreePlantGen/Blueprints/InternalLogic/Tree.Tree_C|SetisUnderWindZoneControl _astree true)))
  ;[0.0244 0.1236 0.41] Let the trees start checking if ON/OFF their wind animation.
  ; It also immediately starts wind animation if they're in range.
  (for _array_element_2 (Variables|Default|GetassignedTrees)
    (Default|CheckingifCullAnimationON/OFF _array_element_2 true))
  (Collision|SetCollisionResponsetoAllChannels (Variables|Default|GetZone) "ECR_Ignore"))

(fn ConstructionScript
  (Components|Sphere|SetSphereRadius (Variables|Default|GetZone) (Variables|Default|GetRadius) false))